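; VR breathing guide ring that paces the player's breathing by growing and shrinking, then returns to the menu.
; Overlap by BP_MyVRPawn reveals BreathRing and plays the RegularBreaths timeline, lerping its scale between StartingScale and EndingScale.
; Delays chained off timeline Update pins start the CoherenceTimer timeline, which drives the same scale, then later hide the ring and open Level_Menu.
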(event `self.BreathRing.OnComponentBeginOverlap`
  (params (OverlappedComponent :type "PrimitiveComponent Object Reference") (OtherActor :type "Actor Object Reference") (OtherComp :type "PrimitiveComponent Object Reference") (OtherBodyIndex :type Integer) (bFromSweep :type Boolean) (SweepResult :type "HitResult Structure (by ref)"))
  (`self.SetActorTickEnabled` true)
  (if (== (`GameplayStatics.GetObjectClass` OtherActor) "/Game/player/BP_MyVRPawn.BP_MyVRPawn_C")
    (`SceneComponent.SetVisibility` (`self.BreathRing`) true false)
    (bind (_direction _regularbreaths) (`Timeline|Regular Breaths`)
      (:`Update`
        (`SceneComponent.SetRelativeScale3D` (`self.BreathRing`) (`KismetMathLibrary.VLerp` (`self.startingScale`) (`self.endingScale`) _regularbreaths))
        (`KismetSystemLibrary.Delay` 10.0)
        (bind (_direction_2 _alpha) (`Timeline|Coherence Timer`)
          (:`Update`
            (`SceneComponent.SetRelativeScale3D` (`self.BreathRing`) (`KismetMathLibrary.VLerp` (`self.startingScale`) (`self.endingScale`) _alpha))
            (`KismetSystemLibrary.Delay` 130.0)
            (`SceneComponent.SetVisibility` (`self.BreathRing`) false false)
            (`KismetSystemLibrary.Delay` 5.0)
            (`GameplayStatics.OpenLevel` "Level_Menu")))))))

(event `self.BreathRing.OnComponentEndOverlap`
  (params (OverlappedComponent :type "PrimitiveComponent Object Reference") (OtherActor :type "Actor Object Reference") (OtherComp :type "PrimitiveComponent Object Reference") (OtherBodyIndex :type Integer)))

(fn `UserConstructionScript`)